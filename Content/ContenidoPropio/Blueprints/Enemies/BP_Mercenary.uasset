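; BP_Mercenary is a mercenary enemy whose Blueprint logic drives an AI debug label showing its role and current state.
; Each Tick reads the MercenaryAIController's blackboard flags in priority order, from reloading and cover through squad tactics to shooting, falling back to moving/searching.
; The resulting Spanish state text is combined with RoleType and written to the WBP_AIDebug widget held by DebugWidget.
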(event `self.ReceiveBeginPlay`)

(event `self.ReceiveTick`
  (params (DeltaSeconds :type "Float (single-precision)"))
  (bind _aswbp_aidebug (cast `/Game/ContenidoPropio/Blueprints/Interface/WBP_AIDebug` (`WidgetComponent.GetUserWidgetObject` (`self.DebugWidget`))))
  (bind _asmercenary_aicontroller (cast `MercenaryAIController` (`self.GetController`)))
  (bind _returnvalue (`AIBlueprintHelperLibrary.GetBlackboard` _asmercenary_aicontroller))
  (if (`BlackboardComponent.GetValueAsBool` _returnvalue "IsReloading")
    (set `self.CurrentState` "Recargando...")
    (elif (`BlackboardComponent.GetValueAsBool` _returnvalue "ShouldCover")
      (set `self.CurrentState` "Cubriéndose")
      (elif (`BlackboardComponent.GetValueAsBool` _returnvalue "IsDefender")
        (set `self.CurrentState` "Defendiendo")
        (elif (`BlackboardComponent.GetValueAsBool` _returnvalue "IsFlanker")
          (set `self.CurrentState` "Flanqueando")
          (elif (`BlackboardComponent.GetValueAsBool` _returnvalue "IsSuppressor")
            (set `self.CurrentState` "Supresion")
            (elif (`BlackboardComponent.GetValueAsBool` _returnvalue "IsInRange")
              (set `self.CurrentState` "Disparando")
              (else
                (set `self.CurrentState` "Moviendose/Buscando"))))))))
  (`TextBlock.SetText` (`/Game/ContenidoPropio/Blueprints/Interface/WBP_AIDebug.DebugText` _aswbp_aidebug) (`|FormatText` "[{Rol}] - {Estado}" (`|GetEnumeratorName` (`self.RoleType`)) (`self.CurrentState`))))

(fn `UserConstructionScript`)